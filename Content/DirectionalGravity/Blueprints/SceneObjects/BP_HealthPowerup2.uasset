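; BP_HealthPowerup2 is a pickup that adds a fixed amount to CurrentHealth when a BP_GravityCharacterBase overlaps its sphere, then destroys itself.
; BeginPlay caches the player pawn and makes the Widget visible.
; The Spin event yaws the Widget toward the player's CameraHolder, billboard-style.
; Spin is bound to a looping zero-second timer, which Unreal treats as a clear, so it does not tick.
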(event `self.ReceiveBeginPlay`
  (`|ExecutionSequence`
    (:`then_0`
      (bind _asbp_gravity_character_base (cast `/Game/DirectionalGravity/Blueprints/GravityLogic/BP_GravityCharacterBase` (`GameplayStatics.GetPlayerPawn` 0)))
      (set `self.PlayerRef` _asbp_gravity_character_base)
      (`SceneComponent.SetVisibility` (`self.Widget`) true false))
    (:`then_1`
      (`KismetSystemLibrary.K2_SetTimerDelegate` (delegate `Spin`) 0.0 true))))

(event `Spin`
  (bind _widget (`self.Widget`))
  (bind (_returnvalue_roll _returnvalue_pitch _returnvalue_yaw) (`KismetMathLibrary.BreakRotator` (`KismetMathLibrary.FindLookAtRotation` (`SceneComponent.K2_GetComponentLocation` _widget) (`SceneComponent.K2_GetComponentLocation` (`/Game/DirectionalGravity/Blueprints/GravityLogic/BP_GravityCharacterBase.CameraHolder` (`self.PlayerRef`))))))
  (`SceneComponent.K2_SetWorldRotation` _widget (`KismetMathLibrary.MakeRotator` 0.0 0.0 _returnvalue_yaw) false false))

(event `self.SphereCollision.OnComponentBeginOverlap`
  (params (OverlappedComponent :type "PrimitiveComponent Object Reference") (OtherActor :type "Actor Object Reference") (OtherComp :type "PrimitiveComponent Object Reference") (OtherBodyIndex :type Integer) (bFromSweep :type Boolean) (SweepResult :type "HitResult Structure (by ref)"))
  (bind _asbp_gravity_character_base (cast `/Game/DirectionalGravity/Blueprints/GravityLogic/BP_GravityCharacterBase` OtherActor))
  (set `/Game/DirectionalGravity/Blueprints/GravityLogic/BP_GravityCharacterBase.CurrentHealth` (+ (`/Game/DirectionalGravity/Blueprints/GravityLogic/BP_GravityCharacterBase.CurrentHealth` _asbp_gravity_character_base) 5.0) _asbp_gravity_character_base)
  (`self.K2_DestroyActor`))

(fn `UserConstructionScript`)