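; BP_EnemyCharger is a robot enemy that charges the player and damages them on contact.
; When PawnSensing sees a BP_GravityCharacterTP, it moves toward that actor with AIMoveTo.
; A Sphere overlap subtracts one CurrentHealth from any BP_GravityCharacterBase.
; Death is checked only on sight events: at zero AIHealth or below, it spawns particles, plays hit and death sounds, and destroys itself.
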(event `self.PawnSensing.OnSeePawn`
  (params (Pawn :type "Pawn Object Reference"))
  (bind _returnvalue (`self.K2_GetActorLocation`))
  (`|ExecutionSequence`
    (:`then_0`
      (bind _asbp_gravity_character_tp (cast `/Game/DirectionalGravity/Blueprints/GravityLogic/BP_GravityCharacterTP` Pawn))
      (`|AIMoveTo` self (0.0 0.0 0.0) _asbp_gravity_character_tp))
    (:`then_1`
      (if (<= (`self.AIHealth`) 0.0)
        (`GameplayStatics.SpawnEmitterAtLocation` "/Game/Particles_Wind_Control_System/Particles/P_Fireflies.P_Fireflies" _returnvalue)
        (`GameplayStatics.PlaySoundAtLocation` "/Game/Sounds/Hit.Hit" _returnvalue (struct) 1.0 1.0 0.0 null null null)
        (`GameplayStatics.PlaySoundAtLocation` "/Game/Sounds/RobotDeath.RobotDeath" _returnvalue (struct) 1.0 1.0 0.0 null null null)
        (`self.K2_DestroyActor`)))))

(event `self.Sphere.OnComponentBeginOverlap`
  (params (OverlappedComponent :type "PrimitiveComponent Object Reference") (OtherActor :type "Actor Object Reference") (OtherComp :type "PrimitiveComponent Object Reference") (OtherBodyIndex :type Integer) (bFromSweep :type Boolean) (SweepResult :type "HitResult Structure (by ref)"))
  (bind _asbp_gravity_character_base (cast `/Game/DirectionalGravity/Blueprints/GravityLogic/BP_GravityCharacterBase` OtherActor))
  (set `/Game/DirectionalGravity/Blueprints/GravityLogic/BP_GravityCharacterBase.CurrentHealth` (- (`/Game/DirectionalGravity/Blueprints/GravityLogic/BP_GravityCharacterBase.CurrentHealth` _asbp_gravity_character_base) 1.0) _asbp_gravity_character_base))

(fn `UserConstructionScript`)