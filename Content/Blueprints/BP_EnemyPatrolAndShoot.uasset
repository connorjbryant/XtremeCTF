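; Robot enemy that shoots the third-person gravity character and damages gravity characters overlapping its sphere.
; PawnSensing turns it toward the seen player and launches a projectile by impulse along the robot's forward vector, throttled by a delay-reset flag.
; BeginPlay stores three patrol points and picks one randomly.
; The timeline logic for lerped patrol movement and zero-health death effects is present but never runs.
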(event `self.PawnSensing.OnSeePawn`
  (params (Pawn :type "Pawn Object Reference"))
  ;[1 1 1] LookAtAndShootPawn
  (bind _asbp_gravity_character_tp (cast `/Game/DirectionalGravity/Blueprints/GravityLogic/BP_GravityCharacterTP` Pawn))
  (`|ExecutionSequence`
    (:`then_0`
      (`self.K2_SetActorRotation` (`KismetMathLibrary.FindLookAtRotation` (`self.K2_GetActorLocation`) (`self.K2_GetActorLocation` _asbp_gravity_character_tp))))
    (:`then_1`
      (if (`self.SpawnProjectile`)
        (bind _returnvalue (`|SpawnActorFromClass` "/Game/FirstPersonBP/Blueprints/FirstPersonProjectile.FirstPersonProjectile_C" (`SceneComponent.K2_GetComponentToWorld` (`self.ProjectileSpawnLocation`)) "Undefined" "OverrideRootScale" null null))
        (`PrimitiveComponent.AddImpulse` (`/Game/FirstPersonBP/Blueprints/FirstPersonProjectile.Sphere` _returnvalue) (* (`SceneComponent.GetForwardVector` (`self.Robot`)) (`self.ShootAmount`)) "None" true)
        (set `self.SpawnProjectile` false)
        (`KismetSystemLibrary.Delay` 1.5)
        (set `self.SpawnProjectile` true)))))

(event `self.ReceiveBeginPlay`
  ;[1 1 1] SetThePatrolPoints
  (set `self.PatrolPoints` (`|MakeArray` (`SceneComponent.K2_GetComponentLocation` (`self.MovePositionOne`)) (`SceneComponent.K2_GetComponentLocation` (`self.MovePositionTwo`)) (`SceneComponent.K2_GetComponentLocation` (`self.MovePositionThree`))))
  (`self.GetRandomLocation`))

(event `self.Sphere.OnComponentBeginOverlap`
  (params (OverlappedComponent :type "PrimitiveComponent Object Reference") (OtherActor :type "Actor Object Reference") (OtherComp :type "PrimitiveComponent Object Reference") (OtherBodyIndex :type Integer) (bFromSweep :type Boolean) (SweepResult :type "HitResult Structure (by ref)"))
  (bind _asbp_gravity_character_base (cast `/Game/DirectionalGravity/Blueprints/GravityLogic/BP_GravityCharacterBase` OtherActor))
  (set `/Game/DirectionalGravity/Blueprints/GravityLogic/BP_GravityCharacterBase.CurrentHealth` (- (`/Game/DirectionalGravity/Blueprints/GravityLogic/BP_GravityCharacterBase.CurrentHealth` _asbp_gravity_character_base) 1.0) _asbp_gravity_character_base))

(fn `GetRandomLocation`
  (set `self.CurrentPatrolPoint` (`KismetMathLibrary.RandomInteger` (`KismetArrayLibrary.Array_Length` (`self.PatrolPoints`)))))

(fn `UserConstructionScript`)