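; NextLevel_BP is a level-exit actor that ends the level once the player has the required item.
; On any actor overlap, it casts the player pawn to BP_GravityCharacterTP and checks that its InventoryItems equals one, without checking which actor overlapped.
; On success it plays a win sound, shows the BPW_NextLevel widget and mouse cursor, then destroys the player character.
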(event `self.ReceiveActorBeginOverlap`
  (params (OtherActor :type "Actor Object Reference"))
  (bind _asbp_gravity_character_tp (cast `/Game/DirectionalGravity/Blueprints/GravityLogic/BP_GravityCharacterTP` (`GameplayStatics.GetPlayerPawn` 0)))
  (if (== (`KismetMathLibrary.Conv_IntToDouble` (`/Game/DirectionalGravity/Blueprints/GravityLogic/BP_GravityCharacterTP.InventoryItems` _asbp_gravity_character_tp)) 1.0)
    (`GameplayStatics.PlaySoundAtLocation` "/Game/Sounds/WIN_sound_effect_no_copyright.WIN_sound_effect_no_copyright" (`self.K2_GetActorLocation` _asbp_gravity_character_tp) (struct) 1.0 1.0 0.0 null null null)
    (bind _returnvalue (`|CreateWidget` "/Game/MenuScreens/BPW_NextLevel.BPW_NextLevel_C"))
    (set `self.NextLevel` _returnvalue)
    (`UserWidget.AddToViewport` _returnvalue 0)
    (set `PlayerController.bShowMouseCursor` true (`GameplayStatics.GetPlayerController` 0))
    (`self.K2_DestroyActor` _asbp_gravity_character_tp)))

(event `self.ReceiveTick`
  (params (DeltaSeconds :type "Float (single-precision)")))

(fn `UserConstructionScript`)