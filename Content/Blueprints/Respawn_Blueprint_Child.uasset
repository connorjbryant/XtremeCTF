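; Respawn trigger child Blueprint that sends a BP_GravityCharacterTP back to a fixed point when it enters the Box volume.
; On begin overlap it sets the character root's relative location to a hard-coded position, then turns on the character's WidgetVisible flag and clears it after a short delay.
; End overlap also clears that flag, and the construction script just calls the parent's.
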(event `self.Box.OnComponentBeginOverlap`
  (params (OverlappedComponent :type "PrimitiveComponent Object Reference") (OtherActor :type "Actor Object Reference") (OtherComp :type "PrimitiveComponent Object Reference") (OtherBodyIndex :type Integer) (bFromSweep :type Boolean) (SweepResult :type "HitResult Structure (by ref)"))
  (bind _asbp_gravity_character_tp (cast `/Game/DirectionalGravity/Blueprints/GravityLogic/BP_GravityCharacterTP` OtherActor))
  (`|ExecutionSequence`
    (:`then_0`
      (`SceneComponent.K2_SetRelativeLocationAndRotation` :`self` (`Actor.RootComponent` _asbp_gravity_character_tp) :`NewLocation` (-5624.955078 18596.441406 11636.726563)))
    (:`then_1`
      (set `/Game/DirectionalGravity/Blueprints/GravityLogic/BP_GravityCharacterTP.WidgetVisible` true _asbp_gravity_character_tp)
      (`KismetSystemLibrary.Delay` 5.0)
      (set `/Game/DirectionalGravity/Blueprints/GravityLogic/BP_GravityCharacterTP.WidgetVisible` false _asbp_gravity_character_tp))))

(event `self.Box.OnComponentEndOverlap`
  (params (OverlappedComponent :type "PrimitiveComponent Object Reference") (OtherActor :type "Actor Object Reference") (OtherComp :type "PrimitiveComponent Object Reference") (OtherBodyIndex :type Integer))
  (bind _asbp_gravity_character_tp (cast `/Game/DirectionalGravity/Blueprints/GravityLogic/BP_GravityCharacterTP` OtherActor))
  (set `/Game/DirectionalGravity/Blueprints/GravityLogic/BP_GravityCharacterTP.WidgetVisible` false _asbp_gravity_character_tp))

(fn `UserConstructionScript`
  (`parent.UserConstructionScript`))